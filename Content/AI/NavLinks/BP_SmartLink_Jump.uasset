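; A smart nav link that makes AI agents jump to the link's destination.
; When an agent reaches the link, it stores the agent and sends it a jump interface message with the link, destination, arc and force multiplier.
; A debug string naming the agent is then printed on screen.
; A call to resume path following is present but unconnected, so the link itself does not resume it.
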(event `self.ReceiveSmartLinkReached`
  (params (Agent :type "Actor Object Reference") (Destination :type "Vector Structure (by ref)"))
  (bind _output_get (set `self.Agent` Agent))
  (message `SmartNavLinkInterface.JumpToDestination` _output_get self Destination (`self.Arc`) (`self.JumpForceMod`))
  (`KismetSystemLibrary.PrintString` (`KismetStringLibrary.Concat_StrStr` (`KismetSystemLibrary.GetDisplayName` (`self.Agent`)) " uses NavLink to Jump!") true true (struct :`R` 1.0 :`G` 0.68703 :`A` 1.0) 10.0))

(fn `UserConstructionScript`)